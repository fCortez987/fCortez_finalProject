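; BP_SniperRound is a sniper projectile that deals damage on overlap with enemies.
; An overlapped BP_Enemy_Base that is not the player pawn receives the round's Damage through ApplyDamage if it has an AC_Health component.
; Unless Piercing is set, the round destroys itself after that hit or on overlap with any non-enemy actor.
; BeginPlay and construction only call the parent class.
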(event `self.ReceiveBeginPlay`
  (`parent.ReceiveBeginPlay`))

(event `self.ReceiveActorBeginOverlap`
  (params (OtherActor :type "Actor Object Reference"))
  (bind _asbp_enemy_base (cast `/Game/Blueprints/Enemies/BP_Enemy_Base` OtherActor)
    (:`then`
      (if (not (== _asbp_enemy_base (`GameplayStatics.GetPlayerPawn` 0)))
        (`/Engine/EditorBlueprintResources/StandardMacros.IsValid` (`self.GetComponentByClass` _asbp_enemy_base "/Game/Blueprints/AC_Health.AC_Health_C")
          (:`Is Valid`
            (`GameplayStatics.ApplyDamage` null (`KismetMathLibrary.Conv_IntToDouble` (`self.Damage`))))
          (:`Is Not Valid`
            _))
        (if (not (`self.Piercing`)) :!label _label
          (`self.K2_DestroyActor`))))
    (:`CastFailed`
      (goto _label))))

(fn `UserConstructionScript`
  (`parent.UserConstructionScript`))