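; BP_FlamePuff is a weapon flame puff whose sphere keeps expanding and damages what it hits.
; From BeginPlay, a self-looping Delay with a short random interval multiplies the sphere's uniform scale, so growth is exponential and unbounded within this graph.
; On Hit, it applies its Damage value to actors with an AC_Health component, skipping the first player's pawn.
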(event `self.ReceiveBeginPlay`
  (bind _sphere (`self.Sphere`))
  (bind _relativescale3d_x (`KismetMathLibrary.BreakVector` (`SceneComponent.RelativeScale3D` _sphere)))
  (bind _returnvalue (* _relativescale3d_x 1.1))
  (`parent.ReceiveBeginPlay`)
  (`KismetSystemLibrary.Delay` (/ 1.0 (`KismetMathLibrary.RandomFloatInRange` 20.0 60.0)) :!label _label)
  (`SceneComponent.SetRelativeScale3D` _sphere (`KismetMathLibrary.MakeVector` _returnvalue _returnvalue _returnvalue))
  (goto _label))

(event `self.ReceiveHit`
  (params (MyComp :type "PrimitiveComponent Object Reference") (Other :type "Actor Object Reference") (OtherComp :type "PrimitiveComponent Object Reference") (bSelfMoved :type Boolean) (HitLocation :type "Vector Structure") (HitNormal :type "Vector Structure") (NormalImpulse :type "Vector Structure") (Hit :type "HitResult Structure (by ref)"))
  (if (not (== Other (`GameplayStatics.GetPlayerPawn` 0)))
    (`/Engine/EditorBlueprintResources/StandardMacros.IsValid` (`self.GetComponentByClass` Other "/Game/Blueprints/AC_Health.AC_Health_C")
      (:`Is Valid`
        (`GameplayStatics.ApplyDamage` Other (`KismetMathLibrary.Conv_IntToDouble` (`self.Damage`)))))))

(fn `UserConstructionScript`
  (`parent.UserConstructionScript`))