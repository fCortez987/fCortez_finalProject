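; BP_GravSniper is a sniper weapon Blueprint that extends a parent weapon class and reloads automatically after every shot.
; Fire runs the parent logic, blocks firing, waits for the modified reload delay, then refills the magazine from reserve ammo, taking only what remains when short.
; The Reload event is overridden as empty, and a debug print stands in for the reload sound.
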(event `self.Fire`
  (bind _ammo_reserves (`self.Ammo Reserves`))
  (bind _returnvalue (- (`self.Mag Size`) (`self.Mag Rounds`)))
  (`parent.Fire`)
  (set `self.Reloading?` true)
  (set `self.Can Fire?` false)
  (`KismetSystemLibrary.PrintString` "[Insert Reloading Noise]")
  (`KismetSystemLibrary.Delay` (* (`self.Reload Delay`) (`self.Reload Mod`)))
  (if (>= _ammo_reserves _returnvalue)
    (set `self.Ammo Reserves` (- _ammo_reserves _returnvalue))
    (set `self.Mag Rounds` (+ (`self.Mag Rounds`) _returnvalue))
    (else
      (set `self.Mag Rounds` (+ (`self.Mag Rounds`) _ammo_reserves))
      (set `self.Ammo Reserves` 0)))
  (set `self.Can Fire?` true)
  (set `self.Reloading?` false))

(event `self.Reload`)

(fn `UserConstructionScript`
  (`parent.UserConstructionScript`))