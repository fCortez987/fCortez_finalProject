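; Shotgun weapon Blueprint that overrides firing and reloading, with print strings standing in for sounds.
; Fire, gated by CanFire, uses one round to spawn a burst of bullets in a loop, then triggers muzzle flash and cooldown.
; Reload blocks firing, waits a modifier-scaled delay, then moves a single round from reserves to the magazine.
; Firing and reloading flags reset only when a round is actually loaded.
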(event `self.Reload`
  (bind _ammo_reserves (`self.Ammo Reserves`))
  (set `self.Reloading?` true)
  (set `self.Can Fire?` false)
  (`KismetSystemLibrary.PrintString` "[Insert Reloading Noise]")
  (`KismetSystemLibrary.Delay` (* (`self.Reload Delay`) (`self.Reload Mod`)))
  (if (and (>= _ammo_reserves 1) (> (- (`self.Mag Size`) (`self.Mag Rounds`)) 0))
    (`/Engine/EditorBlueprintResources/StandardMacros.DecrementInt` _ammo_reserves
      (:`  `
        (`/Engine/EditorBlueprintResources/StandardMacros.IncrementInt` (`self.Mag Rounds`)
          (:`  `
            (set `self.Can Fire?` true)
            (set `self.Reloading?` false)))))))

(event `self.Fire`
  (if (`self.Can Fire?`)
    (`KismetSystemLibrary.PrintString` "[Insert Firing Noise]")
    (`/Engine/EditorBlueprintResources/StandardMacros.DecrementInt` (`self.Mag Rounds`)
      (:`  `
        (for _ (range 11)
          (`self.Spawn Bullet` 30.0))
        (`self.Muzzle Flash`)
        (`self.Firing Cooldown`)))))

(fn `UserConstructionScript`
  (`parent.UserConstructionScript`))