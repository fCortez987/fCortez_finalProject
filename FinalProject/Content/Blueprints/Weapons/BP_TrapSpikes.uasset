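; Spike trap weapon that damages actors, other than the player pawn, that overlap it.
; On BeginPlay it runs the parent logic, then zeroes its projectile movement velocity after a one-second delay.
; Each overlap begin applies its Damage value once, only to actors with an AC_Health component.
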(event `self.ReceiveBeginPlay`
  (`parent.ReceiveBeginPlay`)
  (`KismetSystemLibrary.Delay` 1.0)
  (set `MovementComponent.Velocity` (0.0 0.0 0.0) (`self.ProjectileMovement`)))

(event `self.ReceiveActorBeginOverlap`
  (params (OtherActor :type "Actor Object Reference"))
  (if (not (== OtherActor (`GameplayStatics.GetPlayerPawn` 0)))
    (`/Engine/EditorBlueprintResources/StandardMacros.IsValid` (`self.GetComponentByClass` OtherActor "/Game/Blueprints/AC_Health.AC_Health_C")
      (:`Is Valid`
        (`GameplayStatics.ApplyDamage` OtherActor (`KismetMathLibrary.Conv_IntToDouble` (`self.Damage`)))))))

(fn `UserConstructionScript`
  (`parent.UserConstructionScript`))