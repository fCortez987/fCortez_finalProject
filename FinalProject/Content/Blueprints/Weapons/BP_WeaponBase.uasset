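; BP_WeaponBase is a base weapon Blueprint that handles firing, reloading from reserve ammo, a toggleable laser and muzzle flash.
; Fire spends a round, spawns a bullet at BulletSource, briefly shows a point light and starts a delay-based cooldown via CanFire.
; SpawnBullet accepts a random yaw spread, though Fire passes zero.
; Magazine size scales by the game instance's MagMod on BeginPlay; firing and reload sounds are print-string placeholders.
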(event `self.ReceiveBeginPlay`
  (bind _asgi_syginstance (cast `/Game/Blueprints/GI_SYGInstance` (`GameplayStatics.GetGameInstance`))
    (:`then`
      (set `self.Mag Size` (* (`self.Mag Size`) (`/Game/Blueprints/GI_SYGInstance.Mag Mod` _asgi_syginstance))))
    (:`CastFailed`
      _))
  (set `self.Mag Rounds` (`self.Mag Size`))
  (`SceneComponent.SetVisibility` (`self.PointLight`) false false))

(event `Fire`
  (if (`self.Can Fire?`)
    (`KismetSystemLibrary.PrintString` "[Insert Firing Noise]")
    (`/Engine/EditorBlueprintResources/StandardMacros.DecrementInt` (`self.Mag Rounds`)
      (:`  `
        (`self.Spawn Bullet` 0.0)
        (`self.Muzzle Flash`)
        (`self.Firing Cooldown`)))))

(event `Reload`
  (bind _ammo_reserves (`self.Ammo Reserves`))
  (bind _returnvalue (- (`self.Mag Size`) (`self.Mag Rounds`)))
  (set `self.Reloading?` true)
  (set `self.Can Fire?` false)
  (`KismetSystemLibrary.PrintString` "[Insert Reloading Noise]")
  (`KismetSystemLibrary.Delay` (* (`self.Reload Delay`) (`self.Reload Mod`)))
  (if (>= _ammo_reserves _returnvalue)
    (set `self.Ammo Reserves` (- _ammo_reserves _returnvalue))
    (set `self.Mag Rounds` (+ (`self.Mag Rounds`) _returnvalue))
    (else
      (set `self.Mag Rounds` (+ (`self.Mag Rounds`) _ammo_reserves))
      (set `self.Ammo Reserves` 0)))
  (set `self.Can Fire?` true)
  (set `self.Reloading?` false))

(event `Firing Cooldown`
  (set `self.Can Fire?` false)
  (`KismetSystemLibrary.Delay` (* (`self.Firing Delay`) (`self.Firing Mod`)))
  (set `self.Can Fire?` true))

(event `Toggle Laser`
  (`SceneComponent.ToggleVisibility` (`self.Laser`) true))

(event `Muzzle Flash`
  (bind _pointlight (`self.PointLight`))
  (`SceneComponent.SetVisibility` _pointlight true false)
  (`KismetSystemLibrary.Delay` 0.2)
  (`SceneComponent.SetVisibility` _pointlight false false))

(event `Spawn Bullet`
  (params (Offset :type "Float (double-precision)"))
  (bind _returnvalue (* Offset 0.5))
  (bind _returnvalue_2 (`SceneComponent.K2_GetComponentToWorld` (`self.Bullet Source`)))
  (`|SpawnActorFromClass` (`self.Bullet`) (`KismetMathLibrary.MakeTransform` (.location _returnvalue_2) (`KismetMathLibrary.MakeRotator` (.roll (.rotation _returnvalue_2)) (.pitch (.rotation _returnvalue_2)) (+ (.yaw (.rotation _returnvalue_2)) (`KismetMathLibrary.RandomFloatInRange` (* _returnvalue -1.0) _returnvalue))) (.scale _returnvalue_2)) "AlwaysSpawn" "MultiplyWithRoot" null null))

(fn `UserConstructionScript`)