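; BP_Smg is the automatic submachine gun, a child weapon Blueprint that keeps firing while the player holds the trigger.
; Fire uses a CanFire gate and a delayed loop that spends a round and spawns a bullet until the trigger releases or the magazine empties.
; Reload defers to the parent only when the trigger is released, and ToggleLaser is overridden empty.
; MuzzleFlash only makes the point light visible and is also called at BeginPlay.
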(event `self.ReceiveBeginPlay`
  (`parent.ReceiveBeginPlay`)
  (bind _aspc_stand_your_ground (cast `/Game/Blueprints/PC_StandYourGround` (`GameplayStatics.GetPlayerController` 0)))
  (set `self.Controller Ref` _aspc_stand_your_ground)
  (`self.Muzzle Flash`))

(event `self.Fire`
  (if (`self.Can Fire?`)
    (set `self.Can Fire?` false)
    (if (and (`/Game/Blueprints/PC_StandYourGround.Trigger?` (`self.Controller Ref`)) (> (`self.Mag Rounds`) 0)) :!label _label
      (`/Engine/EditorBlueprintResources/StandardMacros.DecrementInt` (`self.Mag Rounds`)
        (:`  `
          (`self.Spawn Bullet` 17.0)
          (`KismetSystemLibrary.Delay` (`self.Firing Delay`))
          (goto _label)))
      (else
        (set `self.Can Fire?` true)))))

(event `self.Muzzle Flash`
  (`SceneComponent.SetVisibility` (`self.PointLight`) true false))

(event `self.Reload`
  (if (not (`/Game/Blueprints/PC_StandYourGround.Trigger?` (`self.Controller Ref`)))
    (`parent.Reload`)))

(event `self.Toggle Laser`)

(fn `UserConstructionScript`
  (`parent.UserConstructionScript`))