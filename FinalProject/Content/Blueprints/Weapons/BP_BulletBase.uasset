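; Base projectile actor for bullets, with speed, damage and lifetime driven by variables.
; On BeginPlay it applies Velocity to the ProjectileMovement component and starts a delay that destroys it after DespawnTime.
; On hit it ignores the first player's pawn, damages actors with an AC_Health component, spawns a reversed-yaw effect at the impact point and destroys itself.
; Impact particles are still marked TODO for damageable targets.
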(event `self.ReceiveBeginPlay`
  (bind _projectilemovement (`self.ProjectileMovement`))
  (bind _velocity (`self.Velocity`))
  (set `ProjectileMovementComponent.InitialSpeed` _velocity _projectilemovement)
  (set `ProjectileMovementComponent.MaxSpeed` _velocity _projectilemovement)
  (`self.Despawn Timer`))

(event `self.ReceiveHit`
  (params (MyComp :type "PrimitiveComponent Object Reference") (Other :type "Actor Object Reference") (OtherComp :type "PrimitiveComponent Object Reference") (bSelfMoved :type Boolean) (HitLocation :type "Vector Structure") (HitNormal :type "Vector Structure") (NormalImpulse :type "Vector Structure") (Hit :type "HitResult Structure (by ref)"))
  (bind _returnvalue (`KismetMathLibrary.ComposeRotators` (`SceneComponent.K2_GetComponentRotation` MyComp) (`KismetMathLibrary.MakeRotator` 0.0 0.0 180.0)))
  (if (not (== Other (`GameplayStatics.GetPlayerPawn` 0)))
    (`/Engine/EditorBlueprintResources/StandardMacros.IsValid` (`self.GetComponentByClass` Other "/Game/Blueprints/AC_Health.AC_Health_C")
      (:`Is Valid`
        (`GameplayStatics.ApplyDamage` Other (`KismetMathLibrary.Conv_IntToDouble` (`self.Damage`)))
        ;[1 0.7826 0] TODO: Create Impact Particles
        (`NiagaraFunctionLibrary.SpawnSystemAtLocation` null HitLocation _returnvalue))
      (:`Is Not Valid`
        (`NiagaraFunctionLibrary.SpawnSystemAtLocation` null HitLocation _returnvalue)))
    (`self.K2_DestroyActor`)))

(event `Despawn Timer`
  (`KismetSystemLibrary.Delay` (`self.Despawn Time`))
  (`self.K2_DestroyActor`))

(fn `UserConstructionScript`)