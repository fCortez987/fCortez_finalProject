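; BP_AmmoBox is an ammo pickup that refills the reserves of a top-down player character's weapon.
; On actor overlap it casts the other actor to BP_TopDownCharacter and adds two magazines' worth of rounds to that weapon's AmmoReserves, based on its MagSize.
; It then sets a very short lifespan so the box removes itself.
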(event `self.ReceiveActorBeginOverlap`
  (params (OtherActor :type "Actor Object Reference"))
  (bind _weapon (`/Game/Blueprints/BP_TopDownCharacter.Weapon` (`self.Char Ref`)))
  (bind _asbp_top_down_character (cast `/Game/Blueprints/BP_TopDownCharacter` OtherActor))
  (set `self.Char Ref` _asbp_top_down_character)
  (set `/Game/Blueprints/Weapons/BP_WeaponBase.Ammo Reserves` (+ (* (`/Game/Blueprints/Weapons/BP_WeaponBase.Mag Size` _weapon) 2) (`/Game/Blueprints/Weapons/BP_WeaponBase.Ammo Reserves` _weapon)) _weapon)
  (`self.SetLifeSpan` 0.1))

(fn `UserConstructionScript`
  (`parent.UserConstructionScript`))