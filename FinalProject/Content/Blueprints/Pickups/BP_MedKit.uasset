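; BP_MedKit is a health pickup that heals the top-down player character on overlap.
; When a BP_TopDownCharacter overlaps it, it adds its Value to the CurrentHealth on the character's ACHealth component, clamped between zero and MaxHealth and truncated to an integer.
; It then sets a very short lifespan, so it disappears almost immediately after use.
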(event `self.ReceiveActorBeginOverlap`
  (params (OtherActor :type "Actor Object Reference"))
  (bind _ac_health (`/Game/Blueprints/BP_TopDownCharacter.AC_Health` (`self.Char Ref`)))
  (bind _asbp_top_down_character (cast `/Game/Blueprints/BP_TopDownCharacter` OtherActor))
  (set `self.Char Ref` _asbp_top_down_character)
  (set `/Game/Blueprints/AC_Health.Current Health` (`KismetMathLibrary.FTrunc` (`KismetMathLibrary.FClamp` (+ (`/Game/Blueprints/AC_Health.Current Health` _ac_health) (`self.Value`)) 0.0 (`KismetMathLibrary.Conv_IntToDouble` (`/Game/Blueprints/AC_Health.Max Health` _ac_health)))) _ac_health)
  (`self.SetLifeSpan` 0.1))

(fn `UserConstructionScript`
  (`parent.UserConstructionScript`))