(event `self.ReceiveBeginPlay`
  (bind _asgsb_stand_your_ground (cast `/Game/Blueprints/GSB_StandYourGround` (`GameplayStatics.GetGameState`)))
  (set `self.Game State Ref` _asgsb_stand_your_ground)
  (bind _asbp_top_down_character (cast `/Game/Blueprints/BP_TopDownCharacter` (`GameplayStatics.GetPlayerPawn` 0)))
  (set `self.Player Ref` _asbp_top_down_character))

(event `/Game/Blueprints/BPI_Interact.Interacted`
  (if (<= (`/Game/Blueprints/GSB_StandYourGround.Time Left` (`self.Game State Ref`)) 0)
    (`/Engine/EditorBlueprintResources/StandardMacros.DoOnce` false
      (:`Completed`
        (bind (_direction _button_press) (`Timeline|Push`)
          (:`Update`
            (`SceneComponent.K2_AddLocalOffset` (`self.Button`) (`KismetMathLibrary.MakeVector` 0.0 0.0 (/ _button_press 25.0)) false false)
            (`/Game/Blueprints/GSB_StandYourGround.Extraction Timer Tick` (`self.Game State Ref`) (`self.Wait Time`))
            (`/Game/Blueprints/BP_TopDownCharacter.Hide Arrow` (`self.Player Ref`))))))))

(event `self.Capsule.OnComponentBeginOverlap`
  (params (OverlappedComponent :type "PrimitiveComponent Object Reference") (OtherActor :type "Actor Object Reference") (OtherComp :type "PrimitiveComponent Object Reference") (OtherBodyIndex :type Integer) (bFromSweep :type Boolean) (SweepResult :type "HitResult Structure (by ref)"))
  (cast `/Game/Blueprints/BP_TopDownCharacter` OtherActor)
  (`KismetSystemLibrary.PrintString` "test 1")
  (if (`/Game/Blueprints/GSB_StandYourGround.Extract Ready?` (`self.Game State Ref`))
    (`GameplayStatics.SetGamePaused` true)
    (`KismetSystemLibrary.PrintString` "test 2")))

(fn `UserConstructionScript`)