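; Player controller for a top-down shooter that turns Enhanced Input actions into movement, firing and reloading on the possessed BP_TopDownCharacter, cached at BeginPlay.
; Move actions apply swept diagonal local offsets scaled by Speed and SpeedMod on each Ongoing trigger, without delta-time scaling.
; Shooting requires an armed character with rounds in the magazine.
; Reloading requires a non-full magazine and reserve ammo, and the Weapon performs both actions.
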(event `self.ReceiveBeginPlay`
  (bind _asbp_top_down_character (cast `/Game/Blueprints/BP_TopDownCharacter` (`GameplayStatics.GetPlayerPawn` 0)))
  (set `self.Player Ref` _asbp_top_down_character))

(event `EnhancedInput|/Game/Blueprints/Input/IA_MoveUp`
  (params (ActionValue :type Boolean) (ElapsedSeconds :type "Float (double-precision)") (TriggeredSeconds :type "Float (double-precision)") (InputAction :type "InputAction Object Reference" :default "/Game/Blueprints/Input/IA_MoveUp.IA_MoveUp"))
  (bind _returnvalue (* (`self.Speed`) (`self.Speed Mod`)))
  (:`Ongoing`
    (`self.K2_AddActorLocalOffset` (`self.Player Ref`) (`KismetMathLibrary.MakeVector` (* _returnvalue -1.0) _returnvalue) true false)))

(event `EnhancedInput|/Game/Blueprints/Input/IA_MoveDown`
  (params (ActionValue :type Boolean) (ElapsedSeconds :type "Float (double-precision)") (TriggeredSeconds :type "Float (double-precision)") (InputAction :type "InputAction Object Reference" :default "/Game/Blueprints/Input/IA_MoveDown.IA_MoveDown"))
  (bind _returnvalue (* (`self.Speed`) (`self.Speed Mod`)))
  (:`Ongoing`
    (`self.K2_AddActorLocalOffset` (`self.Player Ref`) (`KismetMathLibrary.MakeVector` _returnvalue (* _returnvalue -1.0)) true false)))

(event `EnhancedInput|/Game/Blueprints/Input/IA_MoveLeft`
  (params (ActionValue :type Boolean) (ElapsedSeconds :type "Float (double-precision)") (TriggeredSeconds :type "Float (double-precision)") (InputAction :type "InputAction Object Reference" :default "/Game/Blueprints/Input/IA_MoveLeft.IA_MoveLeft"))
  (bind _returnvalue (* (`self.Speed`) (`self.Speed Mod`)))
  (:`Ongoing`
    (`self.K2_AddActorLocalOffset` (`self.Player Ref`) (`KismetMathLibrary.MakeVector` _returnvalue _returnvalue) true false)))

(event `EnhancedInput|/Game/Blueprints/Input/IA_MoveRight`
  (params (ActionValue :type Boolean) (ElapsedSeconds :type "Float (double-precision)") (TriggeredSeconds :type "Float (double-precision)") (InputAction :type "InputAction Object Reference" :default "/Game/Blueprints/Input/IA_MoveRight.IA_MoveRight"))
  (bind _returnvalue (* (`self.Speed`) (`self.Speed Mod`) -1.0))
  (:`Ongoing`
    (`self.K2_AddActorLocalOffset` (`self.Player Ref`) (`KismetMathLibrary.MakeVector` _returnvalue _returnvalue) true false)))

(event `EnhancedInput|/Game/Blueprints/Input/IA_Shoot`
  (params (ActionValue :type Boolean) (ElapsedSeconds :type "Float (double-precision)") (TriggeredSeconds :type "Float (double-precision)") (InputAction :type "InputAction Object Reference" :default "/Game/Blueprints/Input/IA_Shoot.IA_Shoot"))
  (bind _player_ref (`self.Player Ref`))
  (bind _weapon (`/Game/Blueprints/BP_TopDownCharacter.Weapon` _player_ref))
  (:`Triggered`
    (if (and (`/Game/Blueprints/BP_TopDownCharacter.Armed?` _player_ref) (> (`/Game/Blueprints/BP_WeaponBase.Mag Rounds` _weapon) 0))
      (`/Game/Blueprints/BP_WeaponBase.Fire` _weapon))))

(event `EnhancedInput|/Game/Blueprints/Input/IA_Reload`
  (params (ActionValue :type Boolean) (ElapsedSeconds :type "Float (double-precision)") (TriggeredSeconds :type "Float (double-precision)") (InputAction :type "InputAction Object Reference" :default "/Game/Blueprints/Input/IA_Reload.IA_Reload"))
  (bind _weapon (`/Game/Blueprints/BP_TopDownCharacter.Weapon` (`self.Player Ref`)))
  (:`Triggered`
    (if (and (< (`/Game/Blueprints/BP_WeaponBase.Mag Rounds` _weapon) (`/Game/Blueprints/BP_WeaponBase.Mag Size` _weapon)) (> (`/Game/Blueprints/BP_WeaponBase.Ammo Reserves` _weapon) 0))
      (`/Game/Blueprints/BP_WeaponBase.Reload` _weapon))))

(fn `UserConstructionScript`)