(event `Load Data`
  (bind _aspc_stand_your_ground (cast `/Game/Blueprints/PC_StandYourGround` (`GameplayStatics.GetPlayerController` 0)))
  (set `/Game/Blueprints/PC_StandYourGround.Speed Mod` (`self.Speed Mod`) _aspc_stand_your_ground)
  (bind _asbp_top_down_character (cast `/Game/Blueprints/BP_TopDownCharacter` (`GameplayStatics.GetPlayerPawn` 0)))
  (`|ExecutionSequence`
    (:`then_0`
      (bind _ac_health (`/Game/Blueprints/BP_TopDownCharacter.AC_Health` _asbp_top_down_character))
      (set `/Game/Blueprints/AC_Health.Damage Mod` (`self.Player Damage Mod`) _ac_health)
      (set `/Game/Blueprints/AC_Health.Cooldown Mod` (`self.Cooldown Mod`) _ac_health))
    (:`then_1`
      (bind _output_get (set `self.Weapon` (`self.Weapon`)))
      (`/Game/Blueprints/BP_TopDownCharacter.Equip Weapon` _asbp_top_down_character _output_get)
      (bind _weapon (`/Game/Blueprints/BP_TopDownCharacter.Weapon` _asbp_top_down_character))
      (set `/Game/Blueprints/Weapons/BP_WeaponBase.Firing Mod` (`self.Firing Mod`) _weapon)
      (set `/Game/Blueprints/Weapons/BP_WeaponBase.Reload Mod` (`self.Reload Mod`) _weapon))
    (:`then_2`
      (bind _asgsb_stand_your_ground (cast `/Game/Blueprints/GSB_StandYourGround` (`GameplayStatics.GetGameState`)))
      (set `/Game/Blueprints/GSB_StandYourGround.Money` (`self.Points`) _asgsb_stand_your_ground)
      (set `/Game/Blueprints/GSB_StandYourGround.Money Modifier ` (`self.Points Mod`) _asgsb_stand_your_ground))))

(event `Save Data`
  (`|ExecutionSequence`
    (:`then_0`
      (bind _aspc_stand_your_ground (cast `/Game/Blueprints/PC_StandYourGround` (`GameplayStatics.GetPlayerController` 0)))
      (set `self.Speed Mod` (`/Game/Blueprints/PC_StandYourGround.Speed Mod` _aspc_stand_your_ground)))
    (:`then_1`
      (bind _asbp_top_down_character (cast `/Game/Blueprints/BP_TopDownCharacter` (`GameplayStatics.GetPlayerPawn` 0)))
      (set `self.Health mod` (`/Game/Blueprints/BP_TopDownCharacter.Health Mod` _asbp_top_down_character)))
    (:`then_2`
      (bind _ac_health (`/Game/Blueprints/BP_TopDownCharacter.AC_Health` _asbp_top_down_character))
      (set `self.Player Damage Mod` (`/Game/Blueprints/AC_Health.Damage Mod` _ac_health))
      (set `self.Cooldown Mod` (`/Game/Blueprints/AC_Health.Cooldown Mod` _ac_health)))
    (:`then_3`
      (bind _weapon (`/Game/Blueprints/BP_TopDownCharacter.Weapon` _asbp_top_down_character))
      (set `self.Firing Mod` (`/Game/Blueprints/Weapons/BP_WeaponBase.Firing Mod` _weapon))
      (set `self.Reload Mod` (`/Game/Blueprints/Weapons/BP_WeaponBase.Reload Mod` _weapon))
      (set `self.Weapon` (`GameplayStatics.GetObjectClass` _weapon)))
    (:`then_4`
      (bind _asgsb_stand_your_ground (cast `/Game/Blueprints/GSB_StandYourGround` (`GameplayStatics.GetGameState`)))
      (set `self.Points` (`/Game/Blueprints/GSB_StandYourGround.Money` _asgsb_stand_your_ground))
      (set `self.Points Mod` (`/Game/Blueprints/GSB_StandYourGround.Money Modifier ` _asgsb_stand_your_ground)))))