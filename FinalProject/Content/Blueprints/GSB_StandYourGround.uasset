(event `self.ReceiveBeginPlay`
  (set `self.Time Left` (`self.Survival Time`))
  (`self.Spawn Limit Timer`)
  (bind _asbp_top_down_character (cast `/Game/Blueprints/BP_TopDownCharacter` (`GameplayStatics.GetPlayerPawn` 0)))
  (set `self.Player Ref` _asbp_top_down_character))

(event `Timer Tick`
  (bind _time_left (`self.Time Left`))
  (if (>= (`self.Time Left`) 0) :!label _label
    (`KismetSystemLibrary.Delay` 1.0)
    (`/Engine/EditorBlueprintResources/StandardMacros.DecrementInt` (`self.Time Left`)
      (:`  `
        (set `self.Time Output String` (`KismetStringLibrary.Concat_StrStr` "Survive For " (`KismetStringLibrary.Conv_IntToString` (/ _time_left 60)) "m " (`KismetStringLibrary.Conv_IntToString` (mod _time_left 60)) "s"))
        (goto _label)))
    (else
      (`self.OnTimerEnd`)
      (set `self.Time Output String` "Press The Button!")
      (`self.OnTimerEnd`)
      (`/Game/Blueprints/BP_TopDownCharacter.Show Arrow` (`self.Player Ref`)))))

(event `Change Money`
  (params (`Money Delta` :type Integer))
  (set `self.Money` (+ (* `Money Delta` (`self.Money Modifier `)) (`self.Money`))))

(event `Spawn Limit Timer`
  (`KismetSystemLibrary.Delay` 5.0 :!label _label_2)
  (bind _outactors (`GameplayStatics.GetAllActorsOfClass` "/Game/Blueprints/Enemies/BP_Enemy_Base.BP_Enemy_Base_C"))
  (bind _returnvalue (`KismetArrayLibrary.Array_Length` _outactors))
  (`KismetSystemLibrary.PrintString` (`KismetStringLibrary.Conv_IntToString` _returnvalue))
  (if (>= _returnvalue (`self.Enemy Limit`))
    (set `self.Can Spawn?` false)
    (goto _label_2)
    (else
      (set `self.Can Spawn?` true)
      (goto _label_2))))

(event `Extraction Timer Tick`
  (params (Time :type Integer))
  (bind _time_left (`self.Time Left`))
  (set `self.Time Left` Time)
  (if (> (`self.Time Left`) 0) :!label _label_3
    (`KismetSystemLibrary.Delay` 1.0)
    (`/Engine/EditorBlueprintResources/StandardMacros.DecrementInt` (`self.Time Left`)
      (:`  `
        (set `self.Time Output String` (`KismetStringLibrary.Concat_StrStr` "Extraction Time: " (`KismetStringLibrary.Conv_IntToString` (/ _time_left 60)) "m " (`KismetStringLibrary.Conv_IntToString` (mod _time_left 60)) "s"))
        (goto _label_3)))
    (else
      (`KismetSystemLibrary.PrintString` "Game Over")
      (`self.OnTimerEnd`)
      (set `self.Time Output String` "Extract!")
      (`self.OnTimerEnd`)
      (set `self.Extract Ready?` true)
      (`/Game/Blueprints/BP_TopDownCharacter.Show Arrow` (`self.Player Ref`)))))

(fn `UserConstructionScript`)