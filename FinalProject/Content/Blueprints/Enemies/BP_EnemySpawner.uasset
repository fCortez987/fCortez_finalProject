(event `self.ReceiveBeginPlay`
  (bind (_returnvalue_x _returnvalue_y) (`KismetMathLibrary.BreakVector` (`self.K2_GetActorLocation`)))
  (bind _enemy_types (`self.Enemy Types`))
  (bind _enemy_types_2 (`self.Enemy Types`))
  (bind _spawn_number (`self.Spawn Number`))
  (bind _asgsb_stand_your_ground (cast `/Game/Blueprints/GSB_StandYourGround` (`GameplayStatics.GetGameState`)))
  (set `self.Game State Ref` _asgsb_stand_your_ground)
  (`self.K2_SetActorLocation` (`KismetMathLibrary.MakeVector` _returnvalue_x _returnvalue_y 54.0))
  (if (> _spawn_number 0)
    (for _ (range 1 (+ _spawn_number 1))
      (`|SpawnActorFromClass` (`|GetArrayItem` _enemy_types_2 (`KismetMathLibrary.RandomIntegerInRange` 0 (`KismetArrayLibrary.Array_LastIndex` _enemy_types_2))) (`KismetMathLibrary.Conv_VectorToTransform` (`SceneComponent.K2_GetComponentLocation` (`self.DefaultSceneRoot`))) "AdjustIfPossibleButAlwaysSpawn" "MultiplyWithRoot" null null)
      (`KismetSystemLibrary.Delay` (+ (`self.Spawn Cooldown`) (`self.Cooldown Modifier`))))
    (else
      (if (`/Game/Blueprints/GSB_StandYourGround.Can Spawn?` (`self.Game State Ref`)) :!label _label
        (`|SpawnActorFromClass` (`|GetArrayItem` _enemy_types (`KismetMathLibrary.RandomIntegerInRange` 0 (`KismetArrayLibrary.Array_LastIndex` _enemy_types))) (`KismetMathLibrary.Conv_VectorToTransform` (`SceneComponent.K2_GetComponentLocation` (`self.DefaultSceneRoot`))) "AdjustIfPossibleButAlwaysSpawn" "MultiplyWithRoot" null null)
        (`KismetSystemLibrary.Delay` (+ (`self.Spawn Cooldown`) (`KismetMathLibrary.RandomFloatInRange` 0.0 (`self.Cooldown Modifier`))))
        (goto _label)))))

(fn `UserConstructionScript`)