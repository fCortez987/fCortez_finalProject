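; Base enemy Blueprint that chases the first player's pawn and damages it on contact.
; BeginPlay derives walk and crouch speeds from Speed and its modifier, and Tick reissues AIMoveTo every frame.
; Overlap with BP_TopDownCharacter opens a gate on the move's immediate output, so Attack applies Damage each tick until overlap ends.
; The AttackInterval delay is unconnected, so attacks are not throttled.
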(event `self.ReceiveBeginPlay`
  (bind _charactermovement (`self.CharacterMovement`))
  (bind _output_get (set `CharacterMovementComponent.MaxWalkSpeed` (* (`self.Speed Modifier`) (`self.Speed`)) _charactermovement))
  (set `CharacterMovementComponent.MaxWalkSpeedCrouched` (/ _output_get 2.0) _charactermovement)
  (`|AIMoveTo` self (0.0 0.0 0.0) (`GameplayStatics.GetPlayerPawn` 0) :!label _label
    (:`then`
      (`/Engine/EditorBlueprintResources/StandardMacros.Gate` true :!label _label_2
        (:`Exit`
          (`self.Attack` (stale `self.ReceiveActorBeginOverlap` _asbp_top_down_character)))))))

(event `self.ReceiveTick`
  (params (DeltaSeconds :type "Float (single-precision)"))
  (goto _label))

(event `self.ReceiveActorBeginOverlap`
  (params (OtherActor :type "Actor Object Reference"))
  (bind _asbp_top_down_character (cast `/Game/Blueprints/BP_TopDownCharacter` OtherActor))
  (goto _label_2 :!via `Open`))

(event `self.ReceiveActorEndOverlap`
  (params (OtherActor :type "Actor Object Reference"))
  (cast `/Game/Blueprints/BP_TopDownCharacter` OtherActor)
  (goto _label_2 :!via `Close`))

(event `Attack`
  (params (`Attack Target` :type "Actor Object Reference"))
  (`GameplayStatics.ApplyDamage` `Attack Target` (`self.Damage`)))

(fn `UserConstructionScript`)