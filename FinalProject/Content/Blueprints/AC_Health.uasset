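; Health component that tracks its owner's health, scaling max health by HealthMod when the owner is a BP_TopDownCharacter.
; It binds to the owner's OnTakeAnyDamage, subtracts damage scaled by DamageMod, clamps the result, and fires OnHealthChanged, plus OnHealthDepleted at zero.
; An optional cooldown, scaled by CooldownMod, blocks further damage for a delay after each hit.
; A debug event feeds damage straight into the same handler.
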(event `self.ReceiveBeginPlay`
  (bind _asbp_top_down_character (cast `/Game/Blueprints/BP_TopDownCharacter` (`self.GetOwner`))
    (:`then`
      (bind _output_get (set `self.Player Ref` _asbp_top_down_character))
      (set `self.Max Health` (* (`self.Max Health`) (`/Game/Blueprints/BP_TopDownCharacter.Health Mod` _output_get))))
    (:`CastFailed`
      _))
  (set `self.Current Health` (`self.Max Health`))
  (add `Actor.OnTakeAnyDamage` (`self.GetOwner`) (delegate `OnTakeDamage`)))

(event `OnTakeDamage`
  (params (DamagedActor :type "Actor Object Reference") (Damage :type "Float (single-precision)") (DamageType :type "DamageType Object Reference") (InstigatedBy :type "Controller Object Reference") (DamageCauser :type "Actor Object Reference"))
  (if (`self.Can Be Damaged?`)
    (if (`self.Damage Cooldown?`)
      (`self.Cooldown Update`))
    (bind _output_get (set `self.Current Health` (`KismetMathLibrary.Clamp` (- (`self.Current Health`) (* Damage (`self.Damage Mod`))) 0 (`self.Max Health`))))
    (`self.On Health Changed` _output_get)
    (if (<= (`self.Current Health`) 0)
      (`self.On Health Depleted`))))

(event `Cooldown Update`
  (set `self.Can Be Damaged?` false)
  (`KismetSystemLibrary.Delay` (* (`self.Damage Cooldown`) (`self.Cooldown Mod`)))
  (set `self.Can Be Damaged?` true)
  (`KismetSystemLibrary.PrintString` "Can Be damaged again"))

(event `DEBUG Damage`
  (params (Damage :type "Float (double-precision)"))
  (`self.OnTakeDamage` null Damage))